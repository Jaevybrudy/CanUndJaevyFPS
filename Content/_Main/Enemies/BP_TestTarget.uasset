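; BP_TestTarget is a test dummy enemy that takes hits and respawns in place.
; DummyHit subtracts Damage from Health, prints the health value, and draws the damage amount as red debug text.
; When health would reach zero or below, Death hides the character mesh, waits briefly, then restores full health and shows the mesh again.
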(event `DummyHit`
  (bind _damage (`self.Damage`))
  (`|ExecutionSequence`
    (:`then_0`
      (bind _output_get (set `self.NewHealth` (- (`self.Health`) _damage)))
      (if (<= _output_get 0.0)
        (`self.Death`)
        (else
          (bind _output_get_2 (set `self.Health` _output_get))
          (`KismetSystemLibrary.PrintString` (`KismetStringLibrary.Conv_DoubleToString` _output_get_2) :!label _label))))
    (:`then_1`
      (`KismetSystemLibrary.DrawDebugString` (0.0 0.0 0.0) (`KismetTextLibrary.Conv_TextToString` (`|FormatText` "{Damage}" _damage)) null (struct :`R` 1.0 :`G` 0.079395 :`A` 1.0) 5.0)
      (goto _label))))

(event `Death`
  (`SceneComponent.SetVisibility` (`self.CharacterMesh`) false true)
  (`KismetSystemLibrary.Delay` 0.1)
  (set `self.Health` 100.0)
  (`SceneComponent.SetVisibility` (`self.CharacterMesh`) true true))

(fn `UserConstructionScript`)